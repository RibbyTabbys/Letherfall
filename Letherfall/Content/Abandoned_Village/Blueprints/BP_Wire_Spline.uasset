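; Wire Blueprint for the Abandoned Village that hangs a cable toward a referenced electric pole.
; The Construction Script sets the Cable component's end to the pole's Sphere location, converted into the actor's local space.
; Sag comes from cable gravity scale, either randomized or set by CableHang, and the cable is destroyed when no valid pole is assigned.
; The ResetWire branch and event graph are empty.
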(event EventBeginPlay)

(event Collision|EventActorBeginOverlap
  (params (OtherActor :type Actor%20Object%20Reference)))

(event EventTick
  (params (DeltaSeconds :type Float%20%28single-precision%29)))

(fn ConstructionScript
  (if (Variables|Default|GetReset_Wire)
    _
    (else
      _))
  (Utilities|IsValid (Variables|Default|GetBP_Electric_POle)
    (:Is%20Valid
      (Variables|/Script/CableComponent.CableComponent|SetEndLocation (Variables|Default|GetCable) (Math|Transform|InverseTransformLocation (Transformation|GetActorTransform) (Transformation|GetWorldLocation (Variables|BP_Wire_Spline_C|GetSphere (Variables|Default|GetBP_Electric_POle)))))
      (if (Variables|Default|GetIsRandomHang)
        (Variables|/Script/CableComponent.CableComponent|SetCableGravityScale (Variables|Default|GetCable) (Math|Random|RandomFloatinRange 1.0 2e+01))
        (else
          (Variables|/Script/CableComponent.CableComponent|SetCableGravityScale (Variables|Default|GetCable) (Variables|Default|GetCable_Hang)))))
    (:Is%20Not%20Valid
      (Components|DestroyComponent (Variables|Default|GetCable)))))