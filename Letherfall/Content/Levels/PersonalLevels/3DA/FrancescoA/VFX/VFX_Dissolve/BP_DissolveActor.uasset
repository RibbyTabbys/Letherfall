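; Dissolve VFX actor that animates a skeletal mesh's dissolve alongside a Niagara effect when play begins.
; A shared macro pushes Alpha, edge color and dissolve texture to mesh and Niagara system, creating dynamic material instances, in both the construction script and BeginPlay.
; A timeline then drives Alpha on both to keep them in sync.
; A parallel static mesh macro exists but is not connected.
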(event Custom|Update%20data%20SK
  (Utilities|SKMacro (Variables|Default|GetNiagaraSK) (Variables|Default|GetSkeletalMesh)
    (:Completed
      (bind _newtrack_0 (Timeline|Timeline PlayFromStart)
        (:Update
          (Rendering|Material|SetScalarParameterValueonMaterials (Variables|Default|GetSkeletalMesh) "Alpha" _newtrack_0)
          (Niagara|SetNiagaraVariable(Float) (Variables|Default|GetNiagaraSK) "Alpha" _newtrack_0))))))

(event EventBeginPlay
  (CallFunction|UpdateDataSK))

(fn ConstructionScript
  (Utilities|SKMacro (Variables|Default|GetNiagaraSK) (Variables|Default|GetSkeletalMesh)))