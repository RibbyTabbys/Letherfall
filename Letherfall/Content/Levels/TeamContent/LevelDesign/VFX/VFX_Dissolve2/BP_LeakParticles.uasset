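; BP_LeakParticles is a dissolve effect actor that pairs a skeletal mesh's materials with a Niagara system.
; The construction script applies an Animations value to both, then creates dynamic material instances with a Perlin mask as the dissolve texture.
; On BeginPlay, a timeline drives the mesh's Animations material parameter and the Niagara float together.
; The Niagara variable is named "Animations" at construction but "User_Animation" at runtime.
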(event EventBeginPlay
  (bind _timeline_animation (Timeline|Timeline Play)
    (:Update
      (Rendering|Material|SetScalarParameterValueonMaterials (Variables|Default|GetSkeletalMesh) "Animations" _timeline_animation)
      (Niagara|SetNiagaraVariable(Float) (Variables|Default|GetNiagaraSK) "User_Animation" _timeline_animation))))

(fn ConstructionScript
  (Rendering|Material|SetScalarParameterValueonMaterials (Variables|Default|GetSkeletalMesh) "Animations" (Variables|Default|GetAnimations))
  (Niagara|SetNiagaraVariable(Float) (Variables|Default|GetNiagaraSK) "Animations" (Variables|Default|GetAnimations))
  (for (_array_element _array_index) 0
    (bind _returnvalue (Rendering|Material|CreateDynamicMaterialInstance (Variables|Default|GetSkeletalMesh) _array_index _array_element "None" :!class /Script/Engine.PrimitiveComponent))
    (Rendering|Material|SetTextureParameterValue _returnvalue "Dissolve Texture" "/DatasmithContent/Materials/Water/Textures/T_Perlin_Mask.T_Perlin_Mask")))