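; Enemy character with health and gory per-bone dismemberment; death reduces the player's madness message and destroys the actor.
; Damage drains per-bone durability; depleted bones break their constraint with blood effects, and spine or leg breaks trigger ragdoll.
; A force-driven crawl pulls head and unbroken arms along, but its activation call is disconnected.
; Helpers expose patrol route, movement speed and attack montage with end notification.
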(event Custom|AttackPlayer
  (Animation|Montage|PlayMontage (Variables|Character|GetMesh) 0
    (:OnCompleted
      _)
    (:OnInterrupted
      _))
  (Default|CallOnAttackEnd))

(event EventAddDamage
  (params (Damage :type Float%20%28double-precision%29) (PartDamage :type Integer) (HitBoneName :type Name :default "None") (DamageCauser :type Actor%20Object%20Reference))
  (CallFunction|AnyDamage PartDamage HitBoneName DamageCauser)
  (bind _output_get (Variables|Default|SetHealt (Math|Float|Clamp(Float) (- (Variables|Default|GetHealt) Damage) 0.0 (Variables|Default|GetMaxHealt))))
  (if (<= _output_get 0.0)
    (Class|IMadness|RemoveMadness(Message) (Game|Player|GetPlayerPawn 0) 3e+01)
    (Actor|DestroyActor)))

(event EventTick
  (params (DeltaSeconds :type Float%20%28single-precision%29))
  (bind _mesh (Variables|Character|GetMesh))
  (bind _returnvalue (Transformation|GetSocketLocation _mesh "None"))
  (if (Utilities|Enum|Equal(Enum) (Variables|Default|GetMovementCrawling) "NewEnumerator1")
    (Utilities|FlowControl|Sequence
      (:then_0
        (Utilities|FlowControl|DoOnce false
          (:Completed
            (Utilities|FlowControl|Delay 3.0)
            (goto _label Open))))
      (:then_1
        (Utilities|FlowControl|Gate true :!label _label
          (:Exit
            (CallFunction|SetCapsuleLocation)
            (CallFunction|AddForcetoBone))))
      (:then_2
        (Utilities|FlowControl|Delay 1.0)
        (bind _outhit (Collision|LineTraceByChannel _returnvalue (+ _returnvalue (* "0.000000,0.000000,-1.000000" 1e+03)) "TraceTypeQuery1" false 0 "ForDuration"))
        (Rendering|Decal|SpawnDecalatLocation "/Game/Levels/PersonalLevels/3DA/FrancescoA/Blood/PM_Blood_Decal.PM_Blood_Decal" "-31.500000,-64.000000,-64.000000" (.Location (Collision|BreakHitResult _outhit)) (Math|Conversions|RotationFromXVector (.Normal (Collision|BreakHitResult _outhit))) 6e+01)))))

(event EventGetRefHUD
  (params (Object :type WP%20Main%20Hud%20Object%20Reference))
  (Variables|Default|SetHudRef Object))

(fn ConstructionScript)

(fn AnyDamage
  (params (Damage :type Integer) (HitBoneName :type Name) (DamageCauser :type Actor%20Object%20Reference))
  (Variables|Default|SetApplied%20Damage Damage)
  (Variables|Default|SetHit%20Bone%20Name HitBoneName)
  (Variables|Default|SetDamage%20Causer DamageCauser)
  (CallFunction|RenameBoneName)
  (bind _reachdurabilitylimit (CallFunction|ApplyDamagetoBone))
  (if _reachdurabilitylimit
    (CallFunction|Dismemberment)
    (CallFunction|Physics)))

(fn RenameBoneName
  (switch name (Variables|Default|GetHit%20Bone%20Name)
    (:Pelvis
      _)
    (:Spine_02
      _)
    (:Spine_03
      _)
    (:Neck01
      _)
    (:Head
      _))
  (Variables|Default|SetHit%20Bone%20Name "spine_01"))

(fn ApplyDamagetoBone
  (bind _breakable_bone_durability (Variables|Default|GetBreakable%20Bone/Durability))
  (bind _hit_bone_name (Variables|Default|GetHit%20Bone%20Name))
  (bind (_value _returnvalue) (Utilities|Map|Find _breakable_bone_durability _hit_bone_name))
  (if _returnvalue
    (Utilities|Map|Add (Variables|Default|GetBreakable%20Bone/Durability) (Variables|Default|GetHit%20Bone%20Name) (- _value (Variables|Default|GetApplied%20Damage)))
    (return (<= (.Value (Utilities|Map|Find (Variables|Default|GetBreakable%20Bone/Durability) (Variables|Default|GetHit%20Bone%20Name))) 0))))

(fn Dismemberment
  (bind _hit_bone_name (Variables|Default|GetHit%20Bone%20Name))
  (bind _mesh (Variables|Character|GetMesh))
  (bind _hit_bone_name_2 (Variables|Default|GetHit%20Bone%20Name))
  (bind _mesh_2 (Variables|Character|GetMesh))
  (bind _mesh_3 (Variables|Character|GetMesh))
  (bind _returnvalue (Transformation|GetSocketTransform _mesh _hit_bone_name "RTS_World"))
  (bind _returnvalue_2 (Transformation|GetWorldLocation _mesh_3))
  (Class|SkeletalMeshComponent|BreakConstraint (Variables|Character|GetMesh) (Utilities|CalculateImpulse) (Utilities|GetSocketLocation) _hit_bone_name)
  (Effects|SpawnEmitterAttached "/Game/Levels/PersonalLevels/3DA/FrancescoA/Particles/PS_BloodSpurt.PS_BloodSpurt" _mesh (Variables|Default|GetHit%20Bone%20Name) (.location _returnvalue) (.rotation _returnvalue) "2.000000,2.000000,2.000000" "KeepWorldPosition")
  (Effects|SpawnEmitterAttached "/Game/Levels/PersonalLevels/3DA/FrancescoA/Particles/PS_BloodTrail.PS_BloodTrail" _mesh_2 _hit_bone_name_2 (.location _returnvalue) (.rotation _returnvalue) "1.000000,1.000000,1.000000" "KeepWorldPosition")
  (Effects|SpawnEmitterAttached "/Game/Levels/PersonalLevels/3DA/FrancescoA/Particles/PS_BloodSpurt.PS_BloodSpurt" _mesh_2 _hit_bone_name_2 (.location _returnvalue) (.rotation _returnvalue) "1.000000,1.000000,1.000000" "KeepWorldPosition")
  (Variables|Default|SetHas%20Spine%20Broken (== _hit_bone_name "spine_01"))
  (Utilities|Array|Add (Variables|Default|GetBrokenBones) (Variables|Default|GetHit%20Bone%20Name))
  (bind _outhit (Collision|LineTraceByChannel _returnvalue_2 (+ _returnvalue_2 (* "0.000000,0.000000,-1.000000" 1e+03)) "TraceTypeQuery1" false 0 "None"))
  (Rendering|Decal|SpawnDecalatLocation "/Game/Levels/PersonalLevels/3DA/FrancescoA/Blood/PM_Blood_Decal.PM_Blood_Decal" "-63.000000,-128.000000,-128.000000" (.Location (Collision|BreakHitResult _outhit)) (Math|Conversions|RotationFromXVector (.Normal (Collision|BreakHitResult _outhit))) 6e+01))

(fn ChangeMovementType
  (if (Utilities|Enum|Equal(Enum) (Variables|Default|GetMovementCrawling) "NewEnumerator0")
    (Variables|Default|SetMovementCrawling "NewEnumerator1")))

(fn Physics
  (bind _mesh (Variables|Character|GetMesh))
  (switch name (Variables|Default|GetHit%20Bone%20Name)
    (:Spine_01
      _)
    (:Thigh_R
      _)
    (:Thigh_L
      _)
    (:Calf_R
      _)
    (:Calf_L
      _)
    (:Foot_R
      _)
    (:Foot_L
      _))
  (Physics|SetSimulatePhysics _mesh true)
  (Physics|AddImpulseatLocation _mesh (Utilities|CalculateImpulse) (Utilities|GetSocketLocation) "None")
  (Collision|SetCollisionEnabled (Variables|Collision|GetCapsuleComponent) "NoCollision"))

(fn SetCapsuleLocation
  (Transformation|SetWorldLocation (Variables|Collision|GetCapsuleComponent) (Math|Rotator|GetRotationXVector (Transformation|GetSocketRotation (Variables|Character|GetMesh) "head")) false false))

(fn AddForcetoBone
  (bind _mesh (Variables|Character|GetMesh))
  (Physics|AddForce _mesh (Utilities|CalculateCrawlForce 5e+02 3e+03) "head" true)
  (Utilities|FindBrokenBones (Utilities|Array|MakeArray "upperarm_r" "lowerarm_r" "hand_r")
    (:true
      _)
    (:false
      (Physics|AddForce (Variables|Character|GetMesh) (Utilities|CalculateCrawlForce 1e+03 1e+03) "hand_r" true)))
  (Utilities|FindBrokenBones (Utilities|Array|MakeArray "upperarm_l" "lowerarm_l" "hand_l")
    (:false
      (Physics|AddForce _mesh (Utilities|CalculateCrawlForce 1e+03 1e+03) "hand_l" true))))

(fn GetPatrolRoute
  (return (Variables|AI|GetPatrolRoute)))

(fn SetMovSpeed
  (params (Speed :type E_MovementSpeed%20Enum :default "NewEnumerator0"))
  (bind _output_get (Variables|/Script/Engine.CharacterMovementComponent|SetMaxWalkSpeed (Variables|Character|GetCharacterMovement) (Utilities|Select :Index Speed :NewEnumerator0 0.0 :NewEnumerator1 5e+01 :NewEnumerator2 3e+02 :NewEnumerator3 4.5e+02)))
  (return _output_get))