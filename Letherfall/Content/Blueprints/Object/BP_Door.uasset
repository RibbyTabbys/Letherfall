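; Door actor that swings open when an actor tagged Player overlaps it and closes when that overlap ends.
; On overlap, the player's offset is unrotated into the door's local space, and the sign of X picks which way the door swings.
; A timeline lerps the Door component's relative rotation from its start to the chosen end rotation, and plays in reverse to close.
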(event Custom|Open
  (bind _alpha (Timeline|Timeline Play)
    (:Update
      (Transformation|SetRelativeRotation (Variables|Default|GetDoor) (Math|Rotator|Lerp(Rotator) (Variables|Default|GetStartRot) (Variables|Default|GetEndRot) _alpha) false false))))

(event Custom|Close
  (bind _alpha (Timeline|Timeline Reverse)
    (:Update
      (Transformation|SetRelativeRotation (Variables|Default|GetDoor) (Math|Rotator|Lerp(Rotator) (Variables|Default|GetStartRot) (Variables|Default|GetEndRot) _alpha) false false))))

(event Collision|EventActorEndOverlap
  (params (OtherActor :type Actor%20Object%20Reference))
  (if (Actor|ActorHasTag OtherActor "Player")
    (CallFunction|Close)))

(event Collision|EventActorBeginOverlap
  (params (OtherActor :type Actor%20Object%20Reference))
  (if (Actor|ActorHasTag OtherActor "Player")
    (if (> (.x (Math|Vector|UnrotateVector (- (Transformation|GetActorLocation) (Transformation|GetActorLocation OtherActor)) (Transformation|GetActorRotation))) 0.0)
      (Variables|Default|SetEndRot "0.000000,90.000000,0.000000")
      (else
        (Variables|Default|SetEndRot "0.000000,-90.000000,0.000000")))
    (CallFunction|Open)))

(fn ConstructionScript)